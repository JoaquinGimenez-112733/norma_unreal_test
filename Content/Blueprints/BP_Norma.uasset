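; BP_Norma is a player character that moves along the world X axis, jumps very high and carries a decaying point light.
; BeginPlay adds the Enhanced Input mapping context and raises jump velocity.
; Move input drives movement along X and snaps control rotation to face the travel direction, while jump input starts and stops jumping.
; Each Tick, DecayLighting shifts MaxLighting by a time-scaled decay rate and applies the clamped value as light intensity.
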(event `self.ReceiveBeginPlay`
  (bind _asplayer_controller (cast `PlayerController` (`self.GetController`)))
  (`EnhancedInputSubsystemInterface.AddMappingContext` (pcsubsystem `EnhancedInputLocalPlayerSubsystem` _asplayer_controller) "/Game/Blueprints/Input/IM_Main.IM_Main" 0 (struct))
  (set `CharacterMovementComponent.JumpZVelocity` 3000.0 (`self.CharacterMovement`)))

(event `self.ReceiveTick`
  (params (DeltaSeconds :type "Float (single-precision)"))
  (`self.DecayLighting` DeltaSeconds))

(event `EnhancedInput|/Game/Blueprints/Input/Actions/IA_Jump`
  (params (ActionValue :type Boolean) (ElapsedSeconds :type "Float (double-precision)") (TriggeredSeconds :type "Float (double-precision)") (InputAction :type "InputAction Object Reference" :default "/Game/Blueprints/Input/Actions/IA_Jump.IA_Jump"))
  (:`Started`
    (`self.Jump`))
  (:`Completed`
    (`self.StopJumping`)))

(event `EnhancedInput|/Game/Blueprints/Input/Actions/IA_Move`
  (params (ActionValue :type "Float (double-precision)") (ElapsedSeconds :type "Float (double-precision)") (TriggeredSeconds :type "Float (double-precision)") (InputAction :type "InputAction Object Reference" :default "/Game/Blueprints/Input/Actions/IA_Move.IA_Move"))
  (:`Triggered`
    (`self.AddMovementInput` (3.0 0.0 0.0) ActionValue)
    (`Controller.SetControlRotation` (`self.GetController`) (select `bool` (> ActionValue 0.0) :`false` (`KismetMathLibrary.MakeRotator` 180.0 0.0 180.0) :`true` (`KismetMathLibrary.MakeRotator` 0.0)))))

(fn `DecayLighting`
  (params (A :type "Float (double-precision)"))
  (bind _output_get (set `self.MaxLighting` (+ (`self.MaxLighting`) (* A (`self.LighthingDecay`)))))
  (`LightComponent.SetIntensity` (`self.PointLight`) (`KismetMathLibrary.FClamp` _output_get 0.0 250.0)))

(fn `UserConstructionScript`)